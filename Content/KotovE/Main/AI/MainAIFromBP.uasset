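; AI controller Blueprint that makes a Main_AI pawn wander endlessly between target points.
; On BeginPlay it copies the pawn's target point list, or gathers every TargetPoint in the level when that list is empty.
; Tick calls Patrol, where a flag allows one AIMoveTo at a time and clears on success or failure.
; Each destination is picked at random, though the index range excludes the list's last entry.
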(event Custom|Patrol
  (bind _mytp (Variables|Default|GetMyTP))
  (if (not (Variables|Default|GetOnPatrol))
    (Variables|Default|SetOnPatrol true)
    (AI|AIMoveTo (Variables|Default|GetMy%20Char) "0, 0, 0" (Utilities|Array|Get(acopy) _mytp (Math|Random|RandomInteger (Utilities|Array|LastIndex _mytp))) 5e+01 false
      (:OnSuccess
        _)
      (:OnFail
        _))
    (Variables|Default|SetOnPatrol false)))

(event EventBeginPlay
  (bind _asmain_ai (Utilities|Casting|CastToMain_AI (Pawn|GetControlledPawn)))
  (Variables|Default|SetMy%20Char _asmain_ai)
  (if (<= (Utilities|Array|Length (Variables|/Game/KotovE/Main/Character/Main_AI.Main_AI_C|GetMyTP (Variables|Default|GetMy%20Char))) 0)
    (bind _outactors (Actor|GetAllActorsOfClass "/Script/Engine.TargetPoint"))
    (Variables|Default|SetMyTP _outactors)
    (else
      (Variables|Default|SetMyTP (Variables|/Game/KotovE/Main/Character/Main_AI.Main_AI_C|GetMyTP (Variables|Default|GetMy%20Char))))))

(event EventTick
  (params (DeltaSeconds :type Float%20%28single-precision%29))
  (CallFunction|Patrol))

(fn ConstructionScript)